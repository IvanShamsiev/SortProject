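; SortRange_BP is an actor that generates and owns a centered row of items to be sorted.
; GenerateItems spawns and attaches the actors, derives default size and spacing from the first one's bounds, lays them out along Y in switchable order, then calls an empty random-value hook.
; Destroying the range destroys its items.
; Cast helpers unpack compare, swap and temp-buffer operation objects into their fields, though nothing here calls them.
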(event Custom|DestroySortActors
  (params (DestroyedActor :type Actor%20Object%20Reference))
  (for _array_element (Variables|Default|GetSortActors)
    (Actor|DestroyActor _array_element)))

(event EventBeginPlay
  (Game|BindEventtoOnDestroyed (delegate Custom|DestroySortActors)))

(event Collision|EventActorBeginOverlap
  (params (OtherActor :type Actor%20Object%20Reference)))

(event EventTick
  (params (DeltaSeconds :type Float%20%28single-precision%29)))

(event EventGenerateItems
  (params (ItemClass :type Actor%20Class%20Reference) (Count :type Integer))
  (if (> Count 0)
    (CallFunction|SpawnActors ItemClass Count)
    (CallFunction|PlaceActors)
    (CallFunction|SetActorsRandomValues)))

(fn ConstructionScript)

(fn InitActor
  (params (Actor :type Actor%20Object%20Reference%20%28by%20ref%29))
  (bind _initializedactor (|CallParentFunction Actor))
  (return _initializedactor))

(fn SetDefaultValues
  (params (AverageActor :type Actor%20Object%20Reference))
  (if (Math|Vector|Equal(Vector) (Variables|Default|GetItemSize) "0, 0, 0" 0.0001)
    (Variables|Default|SetItemSize (* (.BoxExtent (Collision|GetActorBounds AverageActor false false)) 2.0))
    (if (== (Variables|Default|GetItemDistance) 0.0)
      (Variables|Default|SetItemDistance (.X (Math|Vector|BreakVector (Variables|Default|GetItemSize)))))))

(fn SpawnActors
  (params (ActorClass :type Actor%20Class%20Reference) (Count :type Integer))
  (for _index (range 1 Count)
    (bind _returnvalue (Game|SpawnActorfromClass ActorClass (Math|Transform|MakeTransform (Transformation|GetActorLocation)) "Undefined" self 0))
    (Transformation|AttachComponentToComponent _returnvalue (Variables|Default|GetDefaultSceneRoot) "None" "KeepRelative" "KeepRelative" "KeepRelative" true)
    (bind _initializedactor (CallFunction|InitActor _returnvalue))
    (Utilities|Array|Add (Variables|Default|GetSortActors) _initializedactor))
  (CallFunction|SetDefaultValues (Utilities|Array|Get(acopy) (Variables|Default|GetSortActors))))

(fn PlaceActors
  (bind _itemsize (Variables|Default|GetItemSize))
  (bind (_x _y _z) (Math|Vector|BreakVector _itemsize))
  (for (_array_element _array_index) (Variables|Default|GetSortActors)
    (Transformation|SetActorRelativeLocation _array_element (Math|Vector|MakeVector 0.0 (* (+ (Math|Conversions|ToFloat(Integer) _array_index) (* (Utilities|Array|Length (Variables|Default|GetSortActors)) -0.5) 0.5) (+ (Variables|Default|GetItemDistance) _y) (Math|Float|SelectFloat 1.0 -1.0 (Variables|Default|GetSwitchItemsOrder))) (/ _z 2.0)))))

(fn SetActorsRandomValues)

(fn CasttoCompare
  (params (SortOperation :type Sort%20Operation%20BP%20Object%20Reference))
  (bind _ascompare_sort_operation_bp (Utilities|Casting|CastToCompareSortOperationBP SortOperation))
  (return (.AsActor (Utilities|Casting|CastToActor (Variables|/Script/SortProject.CompareSortOperationBP|GetFirst _ascompare_sort_operation_bp))) (.AsActor (Utilities|Casting|CastToActor (Variables|/Script/SortProject.CompareSortOperationBP|GetSecond _ascompare_sort_operation_bp))) (Variables|/Script/SortProject.CompareSortOperationBP|GetCompareType _ascompare_sort_operation_bp) (Variables|/Script/SortProject.CompareSortOperationBP|GetCompareSuccess _ascompare_sort_operation_bp)))

(fn CasttoSwap
  (params (SortOperation :type Sort%20Operation%20BP%20Object%20Reference))
  (bind _asswap_sort_operation_bp (Utilities|Casting|CastToSwapSortOperationBP SortOperation))
  (return (.AsActor (Utilities|Casting|CastToActor (Variables|/Script/SortProject.SwapSortOperationBP|GetFirst _asswap_sort_operation_bp))) (.AsActor (Utilities|Casting|CastToActor (Variables|/Script/SortProject.SwapSortOperationBP|GetSecond _asswap_sort_operation_bp)))))

(fn CasttoCreateTemp
  (params (SortOperation :type Sort%20Operation%20BP%20Object%20Reference))
  (bind _ascreate_temp_operation (Utilities|Casting|CastToCreateTempOperation SortOperation))
  (return (Variables|/Script/SortProject.CreateTempOperation|GetTempId _ascreate_temp_operation) (Variables|/Script/SortProject.CreateTempOperation|GetTempSize _ascreate_temp_operation)))

(fn CasttoRemoveTemp
  (params (SortOperation :type Sort%20Operation%20BP%20Object%20Reference))
  (bind _asremove_temp_operation (Utilities|Casting|CastToRemoveTempOperation SortOperation))
  (return (Variables|/Script/SortProject.RemoveTempOperation|GetTempId _asremove_temp_operation)))

(fn CasttoCopytoTemp
  (params (SortOperation :type Sort%20Operation%20BP%20Object%20Reference))
  (bind _ascopy_to_temp_operation (Utilities|Casting|CastToCopyToTempOperation SortOperation))
  (return (.AsActor (Utilities|Casting|CastToActor (Variables|/Script/SortProject.CopyToTempOperation|GetItem _ascopy_to_temp_operation))) (Variables|/Script/SortProject.CopyToTempOperation|GetTempId _ascopy_to_temp_operation) (Variables|/Script/SortProject.CopyToTempOperation|GetTempPosition _ascopy_to_temp_operation)))

(fn CasttoCopyfromTemp
  (params (SortOperation :type Sort%20Operation%20BP%20Object%20Reference))
  (bind _ascopy_from_temp_operation (Utilities|Casting|CastToCopyFromTempOperation SortOperation))
  (return (.AsActor (Utilities|Casting|CastToActor (Variables|/Script/SortProject.CopyFromTempOperation|GetItem _ascopy_from_temp_operation))) (Variables|/Script/SortProject.CopyFromTempOperation|GetTempId _ascopy_from_temp_operation) (Variables|/Script/SortProject.CopyFromTempOperation|GetArrayPosition _ascopy_from_temp_operation)))