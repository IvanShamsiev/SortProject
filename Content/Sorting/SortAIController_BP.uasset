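; AI controller that visualizes a sorting algorithm by animating SortingBox actors in the level.
; On BeginPlay, SortComponent turns the boxes into compare and swap operations, which a custom DelayableForEach loop replays one at a time, advancing when each animation ends.
; Timeline lerps lift and lower each pair: compares spawn a temporary operator text, green or red by result, while swaps move boxes past each other on opposite sideways offsets.
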(event EventBeginPlay
  (bind _outactors (Actor|GetAllActorsOfClass "/Script/SortProject.SortingBox"))
  (bind _resultsbp (Class|SortComponent|StartSorting (Variables|Default|GetSortComponent) _outactors))
  (bind _output_get (Variables|Default|SetResults%20BP _resultsbp))
  (bind _item (Utilities|DelayableforEach _output_get :!label _label)
    (:LoopBody
      (switch Utilities|FlowControl|Switch|SwitchonESortOperationTypeBP (Variables|/Script/SortProject.SortOperationBP|GetType _item)
        (:None
          (Development|PrintString "None!"))
        (:Compare
          (bind (_first _second _compareoperation _comparesuccess) (CallFunction|CasttoCompare _item))
          (|Compare _first _second _compareoperation _comparesuccess
            (:Ok
              (goto _label Next))))
        (:Swap
          (bind (_first_2 _second_2) (CallFunction|CasttoSwap _item))
          (|Swap _first_2 _second_2
            (:Ok
              (goto _label Next))))))))

(event EventTick
  (params (DeltaSeconds :type Float%20%28single-precision%29)))

(fn ConstructionScript)

(fn CasttoCompare
  (params (SortOperation :type Sort%20Operation%20BP%20Object%20Reference))
  (bind _ascompare_sort_operation_bp (Utilities|Casting|CastToCompareSortOperationBP SortOperation))
  (return (.AsSorting%20Box (Utilities|Casting|CastToSortingBox (Variables|/Script/SortProject.CompareSortOperationBP|GetFirst _ascompare_sort_operation_bp))) (.AsSorting%20Box (Utilities|Casting|CastToSortingBox (Variables|/Script/SortProject.CompareSortOperationBP|GetSecond _ascompare_sort_operation_bp))) (Variables|/Script/SortProject.CompareSortOperationBP|GetCompareType _ascompare_sort_operation_bp) (Variables|/Script/SortProject.CompareSortOperationBP|GetCompareSuccess _ascompare_sort_operation_bp)))

(fn CasttoSwap
  (params (SortOperation :type Sort%20Operation%20BP%20Object%20Reference))
  (bind _asswap_sort_operation_bp (Utilities|Casting|CastToSwapSortOperationBP SortOperation))
  (return (.AsSorting%20Box (Utilities|Casting|CastToSortingBox (Variables|/Script/SortProject.SwapSortOperationBP|GetFirst _asswap_sort_operation_bp))) (.AsSorting%20Box (Utilities|Casting|CastToSortingBox (Variables|/Script/SortProject.SwapSortOperationBP|GetSecond _asswap_sort_operation_bp)))))

(fn SetTextParams
  (params (TextRender :type Text%20Render%20Component%20Object%20Reference) (CompareType :type ESortCompareTypeBP%20Enum :default "None") (CompareSuccess :type Boolean))
  (Rendering|Components|TextRender|SetText TextRender (Utilities|Select :Index CompareType :None "" :MoreThan ">" :LessThan "<" :Equals "==" :NotEquals "!="))
  (Rendering|Components|TextRender|SetTextRenderColor TextRender (Math|Conversions|ToColor(LinearColor) (Math|Color|SelectColor "(R=0.000000,G=1.000000,B=0.143351,A=1.000000)" "(R=1.000000,G=0.000000,B=0.006006,A=1.000000)" CompareSuccess)))
  (Rendering|Components|TextRender|SetWorldSize TextRender 5e+01)
  (Rendering|Components|TextRender|SetHorizontalAlignment TextRender "EHTA_Center")
  (Class|TextRenderComponent|SetVerticalAlignment TextRender "EVRTA_TextCenter"))